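; SnowBarrel is a barrel actor whose material snow coverage changes over time while it has nothing overhead.
; Each tick, a short upward Visibility line trace from the barrel mesh, drawn with persistent debug, stops a Timeline on a hit and plays it otherwise.
; The Timeline's Snow track drives the "Snow Amount" material parameter, which the construction script initializes from the SnowAmount variable.
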(event `self.ReceiveBeginPlay`)

(event `self.ReceiveTick`
  (params (DeltaSeconds :type "Float (single-precision)"))
  (bind _returnvalue (`SceneComponent.K2_GetComponentLocation` (`self.SM_Barrel`)))
  (bind (_outhit _returnvalue_2) (`KismetSystemLibrary.LineTraceSingle` :`Start` (+ _returnvalue (0.0 0.0 10.0)) :`End` (+ _returnvalue (0.0 0.0 500.0)) :`TraceChannel` "TraceTypeQuery1" :`DrawDebugType` "Persistent"))
  (if _returnvalue_2
    (bind (_direction _snow) (`Timeline|Timeline` :!via `Stop` :!label _label)
      (:`Update`
        (`MeshComponent.SetScalarParameterValueOnMaterials` (`self.SM_Barrel`) "Snow Amount" _snow)))
    (else
      (goto _label))))

(event `self.ReceiveActorOnClicked`
  (params (ButtonPressed :type "Key Structure")))

(fn `UserConstructionScript`
  (`MeshComponent.SetScalarParameterValueOnMaterials` (`self.SM_Barrel`) "Snow Amount" (`self.Snow Amount`)))